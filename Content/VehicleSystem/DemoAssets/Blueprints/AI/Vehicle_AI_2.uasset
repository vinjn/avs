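; AI controller that drives a possessed AVS vehicle along AI_SplinePath waypoints, starting from the nearest path.
; A looping timer steers by yaw to the current waypoint and sets throttle and brake toward a target speed lowered for current and upcoming turns.
; Non-looping paths hand off to a random connected path or stop with handbrake.
; Vehicle_DemoBase repairs are requested after prolonged rollover or without a working drive wheel at start-up.
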(event Custom|ReadyUpVehicle
  (bind _controlledvehicle (Variables|Default|GetControlledVehicle))
  (Utilities|IsValid _controlledvehicle
    (:Is%20Valid
      (Default|StartEngine _controlledvehicle)
      (Default|SetShifterPosition _controlledvehicle "NewEnumerator3")
      (if (not (CallFunction|GetHasActiveDrivingWheel _controlledvehicle))
        (bind _asvehicle_demo_base (Utilities|Casting|CastToVehicle_DemoBase _controlledvehicle))
        (Default|RequestFixVehicle _asvehicle_demo_base)))))

(event Custom|UnStuck
  (Utilities|Time|ClearandInvalidateTimerbyHandle (Variables|Default|GetStuckTimer))
  (bind _asvehicle_demo_base (Utilities|Casting|CastToVehicle_DemoBase (Variables|Default|GetControlledVehicle)))
  (Default|RequestFixVehicle _asvehicle_demo_base))

(event EventUnPossess
  (params (UnpossessedPawn :type Pawn%20Object%20Reference))
  (Utilities|Time|ClearandInvalidateTimerbyHandle (Variables|Default|GetLocationTick))
  (Utilities|Time|ClearandInvalidateTimerbyHandle (Variables|Default|GetReadyTimer))
  (Variables|Default|SetControlledVehicle 0))

(event EventTick
  (params (DeltaSeconds :type Float%20%28single-precision%29))
  (bind _controlledvehicle (Variables|Default|GetControlledVehicle))
  (Utilities|IsValid _controlledvehicle
    (:Is%20Valid
      (if (> (Math|Float|Absolute(Float) (.Roll (Math|Rotator|BreakRotator (Transformation|GetActorRotation _controlledvehicle)))) 6e+01)
        (if (not (Utilities|Time|IsTimerActivebyHandle (Variables|Default|GetStuckTimer)))
          (bind _returnvalue (Utilities|Time|SetTimerbyEvent (delegate Custom|UnStuck) 5.0))
          (Variables|Default|SetStuckTimer _returnvalue))
        (elif (Utilities|Time|IsTimerActivebyHandle (Variables|Default|GetStuckTimer))
          (Utilities|Time|ClearandInvalidateTimerbyHandle (Variables|Default|GetStuckTimer)))))))

(event EventPossess
  (params (PossessedPawn :type Pawn%20Object%20Reference))
  (bind _asavs_vehicle (Utilities|Casting|CastToAVS_Vehicle PossessedPawn))
  (Variables|Default|SetControlledVehicle _asavs_vehicle)
  (bind _returnvalue (Utilities|Time|SetTimerbyEvent (delegate Custom|ReadyUpVehicle) 0.5))
  (Variables|Default|SetReadyTimer _returnvalue)
  (bind _nearestpath (CallFunction|GetNearestPath))
  (Commands|StartMovement _nearestpath))

(fn ConstructionScript)

(fn StartMovement
  (params (Path :type AI%20Spline%20Path%20Object%20Reference) (Waypoint :type Integer))
  (bind _output_get (LocalVariables|SetLastPath (Variables|Default|GetCurrentPath)))
  (LocalVariables|SetSelectNextPath (or (not (Utilities|IsValid (Variables|Default|GetCurrentPath))) (!= _output_get Path)))
  (bind _output_get_2 (Variables|Default|SetCurrentPath Path))
  (Utilities|IsValid _output_get_2
    (:Is%20Valid
      (Variables|Default|SetCurrentWaypoint Waypoint)
      (Default|SetHandbrakeInput (Variables|Default|GetControlledVehicle) false)
      (bind _returnvalue (Utilities|Time|SetTimerbyFunctionName 0 "UpdateMovement" 0.03 true))
      (Variables|Default|SetLocationTick _returnvalue)
      (if (LocalVariables|GetSelectNextPath)
        (if (not (Variables|/Game/VehicleSystem/DemoAssets/Blueprints/AI/AI_SplinePath.AI_SplinePath_C|GetLoop (Variables|Default|GetCurrentPath)))
          ;[1 1 1] Randomly select a connected path
          (LocalVariables|SetAvailablePaths (Variables|/Game/VehicleSystem/DemoAssets/Blueprints/AI/AI_SplinePath.AI_SplinePath_C|GetConnectedPaths (Variables|Default|GetCurrentPath)))
          (Utilities|Array|RemoveItem (LocalVariables|GetAvailablePaths) (LocalVariables|GetLastPath))
          (if (Utilities|Array|IsValidIndex (LocalVariables|GetAvailablePaths) (Math|Random|RandomIntegerinRange 0 (Utilities|Array|LastIndex (LocalVariables|GetAvailablePaths))))
            (Variables|Default|SetNextPath (Utilities|Array|Get(acopy) (LocalVariables|GetAvailablePaths) (Math|Random|RandomIntegerinRange 0 (Utilities|Array|LastIndex (LocalVariables|GetAvailablePaths)))))))))))

(fn UpdateMovement
  (bind _speedtarget (Variables|Default|GetSpeedTarget))
  (bind _controlledvehicle (Variables|Default|GetControlledVehicle))
  (bind _speedtarget_2 (Variables|Default|GetSpeedTarget))
  (bind _controlledvehicle_2 (Variables|Default|GetControlledVehicle))
  (bind _output_get (Variables|Default|SetCurrentDistance (Utilities|GetDistancetoDestination)))
  (if (> _output_get 8e+02)
    (Runtime|CalculateSpeed)
    (Runtime|CalculateSteering)
    ;[1 1 1] Maintain Speed and Apply Steering
    (Default|SetThrottleInput _controlledvehicle_2 (Math|Float|MapRangeClamped (Default|GetAirSpeed _controlledvehicle_2) (- _speedtarget_2 1e+01) _speedtarget_2 1.0 0.0))
    (Default|SetBrakeInput _controlledvehicle (Math|Float|MapRangeClamped (Default|GetAirSpeed _controlledvehicle) (+ _speedtarget 1.0) (+ _speedtarget 1e+01) 0.0 1.0))
    (Default|SetSteeringInput _controlledvehicle (Variables|Default|GetSteeringTarget))
    (else
      (Runtime|ArriveatDestination))))

(fn CalculateSteering
  (Variables|Default|SetSteeringTarget (Math|Float|MapRangeUnclamped (CallFunction|GetDirtoWaypoint (CallFunction|GetCurrentWaypoint)) -45.0 45.0 -1.0 1.0))
  (return))

(fn CalculateSpeed
  (bind _turnevaldistance (Variables|Config|GetTurnEvalDistance))
  (bind (_path _pointindex) (CallFunction|GetNextWaypoint))
  (Variables|Default|SetSpeedTarget (Math|Float|MapRangeClamped (Math|Float|Max(Float) (Math|Float|Absolute(Float) (CallFunction|GetDirtoWaypoint (CallFunction|GetCurrentWaypoint))) (Math|Float|MapRangeClamped (Variables|Default|GetCurrentDistance) (Math|Conversions|ToFloat(Integer) _turnevaldistance) (Math|Conversions|ToFloat(Integer) (+ _turnevaldistance 1000)) (Math|Float|Absolute(Float) (CallFunction|GetDirtoWaypoint (Utilities|Array|Get(acopy) (Variables|/Game/VehicleSystem/DemoAssets/Blueprints/AI/AI_SplinePath.AI_SplinePath_C|GetPoints _path) _pointindex))) 0.0)) 0.0 9e+01 (Math|Conversions|ToFloat(Integer) (Variables|Config|GetMaxSpeed)) (Math|Conversions|ToFloat(Integer) (Variables|Config|GetHighRiskTurnSpeed))))
  (return))

(fn ArriveatDestination
  (bind _controlledvehicle (Variables|Default|GetControlledVehicle))
  (bind _currentpath (Variables|Default|GetCurrentPath))
  (Utilities|Time|ClearandInvalidateTimerbyHandle (Variables|Default|GetLocationTick))
  (bind (_path _pointindex) (CallFunction|GetNextWaypoint))
  (if (!= _path (Variables|Default|GetCurrentPath))
    (Variables|Default|SetNextPath 0)
    (Commands|StartMovement _path _pointindex)
    (elif (== _pointindex 0)
      (if (Variables|/Game/VehicleSystem/DemoAssets/Blueprints/AI/AI_SplinePath.AI_SplinePath_C|GetLoop _currentpath)
        (Commands|StartMovement _currentpath)
        (else
          ;[1 1 1] Stop Vehicle
          (Default|SetThrottleInput _controlledvehicle 0.0)
          (Default|SetBrakeInput _controlledvehicle 0.0)
          (Default|SetHandbrakeInput _controlledvehicle true)))
      (else
        (Commands|StartMovement _path _pointindex)))))

(fn GetNearestPath
  (bind _returnvalue (Pawn|GetControlledPawn))
  (bind _outactors (Actor|GetAllActorsOfClass "/Game/VehicleSystem/DemoAssets/Blueprints/AI/AI_SplinePath.AI_SplinePath_C"))
  (for _array_element _outactors
    (Utilities|IsValid _returnvalue
      (:Is%20Valid
        (Utilities|IsValid _array_element
          (:Is%20Valid
            (if (or (< (Math|Vector|Distance2D(Vector) (Transformation|GetActorLocation _returnvalue) (Transformation|GetActorLocation _array_element)) (LocalVariables|GetBestDistance)) (== (LocalVariables|GetBestDistance) 0.0))
              (LocalVariables|SetSelectedPath _array_element)
              (LocalVariables|SetBestDistance (Math|Vector|Distance2D(Vector) (Transformation|GetActorLocation _returnvalue) (Transformation|GetActorLocation _array_element)))))))))
  (return (LocalVariables|GetSelectedPath)))

(fn GetCurrentWaypoint
  (return (Utilities|Array|Get(acopy) (Variables|/Game/VehicleSystem/DemoAssets/Blueprints/AI/AI_SplinePath.AI_SplinePath_C|GetPoints (Variables|Default|GetCurrentPath)) (Variables|Default|GetCurrentWaypoint))))

(fn GetNextWaypoint
  (bind _currentwaypoint (Variables|Default|GetCurrentWaypoint))
  (bind _nextpath (Variables|Default|GetNextPath))
  (bind _currentpath (Variables|Default|GetCurrentPath))
  (bind _returnvalue (+ _currentwaypoint 1))
  (bind _point_index (CallFunction|GetPathWaypoint _currentpath _returnvalue))
  (if (and (== _point_index 0) (not (Variables|/Game/VehicleSystem/DemoAssets/Blueprints/AI/AI_SplinePath.AI_SplinePath_C|GetLoop _currentpath)))
    (Utilities|IsValid _nextpath
      (:Is%20Valid
        (return _nextpath (.Point%20Index (CallFunction|GetPathWaypoint _nextpath))))
      (:Is%20Not%20Valid
        _)))
  (return (Variables|Default|GetCurrentPath) _point_index))

(fn GetDirtoWaypoint
  (params (PointLocation :type Vector))
  (bind (_x _y) (Math|Vector|BreakVector PointLocation))
  (bind _controlledvehicle (Variables|Default|GetControlledVehicle))
  (bind _returnvalue (Transformation|GetActorLocation _controlledvehicle))
  (return (Math|Float|Clamp(Float) (.yaw (Math|Rotator|Delta(Rotator) (Math|Rotator|FindLookatRotation (Math|Vector|MakeVector (.x _returnvalue) (.y _returnvalue) 0.0) (Math|Vector|MakeVector _x _y 0.0)) (Transformation|GetActorRotation _controlledvehicle))) -9e+01 9e+01)))

(fn GetPathWaypoint
  (params (Path :type AI%20Spline%20Path%20Object%20Reference) (PointIndex :type Integer))
  (bind _points (Variables|/Game/VehicleSystem/DemoAssets/Blueprints/AI/AI_SplinePath.AI_SplinePath_C|GetPoints Path))
  (if (<= PointIndex (Utilities|Array|LastIndex _points))
    (return (Utilities|Array|Get(acopy) _points PointIndex) PointIndex)
    (else
      (return (Utilities|Array|Get(acopy) _points) 0))))

(fn GetHasActiveDrivingWheel
  (params (Vehicle :type AVS%20Vehicle%20Object%20Reference))
  (bind _array_element (Utilities|Array|ForEachLoopwithBreak (Default|GetAllWheels Vehicle) :!label _label)
    (:LoopBody
      (if (and (Variables|/VehicleSystemPlugin/VehicleAssets/Components/Vehicle_Wheel.Vehicle_Wheel_C|GetisDrivingWheel _array_element) (Default|GetIsConstrained _array_element))
        (LocalVariables|SetHasWorkingDrivingWheel true)
        (goto _label Break)))
    (:Completed
      (return (LocalVariables|GetHasWorkingDrivingWheel)))))