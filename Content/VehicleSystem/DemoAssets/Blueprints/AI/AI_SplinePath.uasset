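; AI path actor for the vehicle system that acts as either a single waypoint or a multi-point spline, linked through ConnectedPaths.
; The construction script caches world locations in Points, destroying the spline for waypoints or making it linear and optionally looped.
; It also builds visual link arrows: waypoints point to every connection or turn red when unlinked, while splines point from their last point to the first connection.
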(fn ConstructionScript
  (bind _returnvalue (Transformation|GetActorLocation))
  (bind _spline (Variables|Default|GetSpline))
  (bind _connectedpaths (Variables|Config|GetConnectedPaths))
  (bind _spline_2 (Variables|Default|GetSpline))
  (bind _spline_3 (Variables|Default|GetSpline))
  (bind _connectedpaths_2 (Variables|Config|GetConnectedPaths))
  (bind _returnvalue_2 (Spline|GetNumberOfSplinePoints _spline_3))
  (bind _returnvalue_3 (- _returnvalue_2 1))
  (bind _returnvalue_4 (Spline|GetLocationatSplinePoint _spline_3 _returnvalue_3 "World"))
  (Utilities|Array|Clear (Variables|Default|GetPoints))
  (Collision|SetActorEnableCollision false)
  (if (Variables|Config|GetIsWaypoint)
    (Utilities|Array|Add (Variables|Default|GetPoints) (Transformation|GetActorLocation))
    (Variables|Config|SetLoop false)
    (Components|DestroyComponent (Variables|Default|GetSpline))
    (if (Utilities|Array|IsValidIndex _connectedpaths)
      (for _array_element _connectedpaths
        (Utilities|IsValid _array_element
          (:Is%20Valid
            (Utilities|FlowControl|Sequence
              (:then_0
                (bind _returnvalue_5 (AddComponent|AddStaticMeshComponent false))
                (Components|StaticMesh|SetStaticMesh _returnvalue_5 "/Engine/VREditor/TransformGizmo/TranslateArrowHandle.TranslateArrowHandle")
                (Transformation|SetWorldRotation _returnvalue_5 (Math|Rotator|FindLookatRotation (Math|Vector|MakeVector (.x _returnvalue) (.y _returnvalue) 0.0) (Math|Vector|MakeVector (.x (Transformation|GetActorLocation _array_element)) (.y (Transformation|GetActorLocation _array_element)) 0.0)) false false)
                (Transformation|SetRelativeScale3D _returnvalue_5 "50.000000,50.000000,50.000000")
                (Rendering|Material|SetMaterial _returnvalue_5 1 "/Game/VehicleSystem/DemoAssets/Materials/Colors/Color_Yellow.Color_Yellow")
                (Development|SetHiddeninGame _returnvalue_5 true false))))))
      (else
        ;[1 0 0] No Connected Paths
        (bind _returnvalue_6 (AddComponent|AddStaticMeshComponent false (Math|Transform|MakeTransform "0, 0,1000.000000" "-90.000000, 0, 0" "20.000000,20.000000,20.000000")))
        (Components|StaticMesh|SetStaticMesh _returnvalue_6 "/Engine/VREditor/TransformGizmo/TranslateArrowHandle.TranslateArrowHandle")
        (Rendering|Material|SetMaterial _returnvalue_6 1 "/Game/VehicleSystem/DemoAssets/Vehicles/Common/Debug/Color_Red_Fullbright.Color_Red_Fullbright")
        (Rendering|Material|SetMaterial (Variables|Default|GetWaypoint) 0 "/Game/VehicleSystem/DemoAssets/Vehicles/Common/Debug/Color_Red_Fullbright.Color_Red_Fullbright")))
    (else
      (for _index (range 0 (- (Spline|GetNumberOfSplinePoints _spline) 1))
        (Utilities|Array|Add (Variables|Default|GetPoints) (Spline|GetLocationatSplinePoint _spline _index "World"))
        (Spline|SetSplinePointType (Variables|Default|GetSpline) _index "Linear" true))
      (Utilities|IsValid _spline_2
        (:Is%20Valid
          (Spline|SetClosedLoop _spline_2 (Variables|Config|GetLoop) true)
          ;[1 1 1] Spline Arrows
          (for _array_element_2 (Variables|Config|GetConnectedPaths)
            _)
          (if (Utilities|Array|IsValidIndex _connectedpaths_2)
            (bind _returnvalue_7 (AddComponent|AddStaticMeshComponent false))
            (Components|StaticMesh|SetStaticMesh _returnvalue_7 "/Engine/VREditor/TransformGizmo/TranslateArrowHandle.TranslateArrowHandle")
            (Transformation|SetWorldTransform _returnvalue_7 (Math|Transform|MakeTransform (+ _returnvalue_4 "0, 0,500.000000") (Math|Rotator|FindLookatRotation _returnvalue_4 (Transformation|GetActorLocation (Utilities|Array|Get(acopy) _connectedpaths_2))) "25.000000,25.000000,25.000000") false false)
            (Rendering|Material|SetMaterial _returnvalue_7 1 "/Game/VehicleSystem/DemoAssets/Materials/Colors/Color_Yellow.Color_Yellow")))))))